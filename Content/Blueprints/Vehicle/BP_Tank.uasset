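; BP_Tank is a drivable tank pawn using Enhanced Input to steer, move and rotate its cabin independently.
; Pressing F spawns a BP_Bullet at BulletArrow with a world camera shake, and releasing it stops all shakes.
; The interact action exits the tank by unhiding the BP_CharacterWASD actor, moving it to SpawnPoint and having the player controller possess it again.
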(event Input|EnhancedActionEvents|EnhancedInputActionIA_VEH_Interact
  (params (ActionValue :type Boolean) (ElapsedSeconds :type Float%20%28double-precision%29) (TriggeredSeconds :type Float%20%28double-precision%29) (InputAction :type Input%20Action%20Object%20Reference :default "/Game/Blueprints/Vehicle/IA_VEH_Interact.IA_VEH_Interact"))
  (bind _spawnpoint (Variables|Default|GetSpawnPoint))
  (bind _returnvalue (Transformation|GetWorldTransform _spawnpoint))
  ;[0.15 0.15 0.15 0.5] SALIR TANQUE
  (:Started
    (bind _returnvalue_2 (Actor|GetActorOfClass "/Game/Blueprints/Character/BP_CharacterWASD.BP_CharacterWASD_C"))
    (Rendering|SetActorHiddenInGame _returnvalue_2 false)
    (Transformation|SetActorTransform _returnvalue_2 (Math|Transform|MakeTransform (.location _returnvalue) (.rotation _returnvalue) "1.000000,1.000000,1.000000"))
    (Pawn|Possess (Game|GetPlayerController 0) _returnvalue_2)))

(event Input|EnhancedActionEvents|EnhancedInputActionIA_VEH_Movement
  (params (ActionValue :type Vector%202D%20Structure) (ElapsedSeconds :type Float%20%28double-precision%29) (TriggeredSeconds :type Float%20%28double-precision%29) (InputAction :type Input%20Action%20Object%20Reference :default "/Game/Blueprints/Vehicle/IA_VEH_Movement.IA_VEH_Movement"))
  ;[0.15 0.15 0.15 0.5] MOVIMIENTO TANQUE
  (Pawn|Input|AddControllerYawInput (.x ActionValue))
  (Pawn|Input|AddMovementInput (Math|Vector|GetForwardVector (Math|Rotator|MakeRotator 0.0 0.0 (.yaw (Pawn|GetControlRotation :!class /Script/Engine.Pawn)))) (* (.y ActionValue) (Variables|Default|GetvehicleMovSpeed)) false))

(event Input|EnhancedActionEvents|EnhancedInputActionIA_VEH_Point
  (params (ActionValue :type Vector%202D%20Structure) (ElapsedSeconds :type Float%20%28double-precision%29) (TriggeredSeconds :type Float%20%28double-precision%29) (InputAction :type Input%20Action%20Object%20Reference :default "/Game/Blueprints/Vehicle/IA_VEH_Point.IA_VEH_Point"))
  ;[0.15 0.15 0.15 0.5] ROTAR CABINA
  (Transformation|AddWorldRotation (Variables|Default|GetCABINA) (Math|Rotator|MakeRotator 0.0 0.0 (.x ActionValue)) false false))

(event Input|KeyboardEvents|F
  (params (Key :type Key%20Structure :default "None"))
  ;[0.15 0.15 0.15 0.5] Logica_Disparar
  (:Pressed
    (CallFunction|Shoot)
    (Camera|PlayWorldCameraShake "/Game/Blueprints/BP_CameraShakeISO.BP_CameraShakeISO_C" (Transformation|GetActorLocation) 0.0 1e+04 0.0))
  (:Released
    (CameraShake|StopAllCameraShakes (Game|GetPlayerCameraManager 0) false)))

(fn ConstructionScript)

(fn Shoot
  ;[0.15 0.15 0.15 0.5] CONSTRUCT BULLET
  (Game|SpawnActorfromClass "/Game/Blueprints/BP_Bullet.BP_Bullet_C" (Math|Transform|MakeTransform (Transformation|GetWorldLocation (Variables|Default|GetBullet_Arrow)) (Transformation|GetWorldRotation (Variables|Default|GetBullet_Arrow)) "1.000000,1.000000,1.000000") "Undefined" "MultiplyWithRoot" 0 0))