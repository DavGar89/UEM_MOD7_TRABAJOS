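; BP_Bullet is a projectile actor that flies straight along its forward vector.
; Tick moves it by Speed scaled by delta time, without sweep, then runs into a five-second Delay that destroys it, acting as a lifetime limit.
; An overlap on its Collision component destroys the bullet early when the other actor is a BP_Cube, leaving the cube untouched here.
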(event OnComponentBeginOverlap(Collision)
  (params (OverlappedComponent :type Primitive%20Component%20Object%20Reference) (OtherActor :type Actor%20Object%20Reference) (OtherComp :type Primitive%20Component%20Object%20Reference) (OtherBodyIndex :type Integer) (bFromSweep :type Boolean) (SweepResult :type Hit%20Result%20Structure%20%28by%20ref%29))
  ;[0.15 0.15 0.15 0.5] Destruccion_Bala_Colision
  (Utilities|Casting|CastToBP_Cube OtherActor)
  (Actor|DestroyActor))

(event EventTick
  (params (DeltaSeconds :type Float%20%28single-precision%29))
  ;[0.15 0.15 0.15 0.5] Creacion_Bala_Al_Disparar
  (Transformation|SetActorLocation (+ (* (* (Transformation|GetActorForwardVector) (Variables|Default|GetSpeed)) DeltaSeconds) (Transformation|GetActorLocation)) false false)
  ;[0.15 0.15 0.15 0.5] DESTRUCCION BALA
  (Utilities|FlowControl|Delay 5.0)
  (Actor|DestroyActor))

(fn ConstructionScript)