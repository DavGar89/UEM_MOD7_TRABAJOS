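; Player character with Enhanced Input movement, look, jump, spring-arm zoom, and running that raises walk speed with a camera shake.
; Interact possesses an overlapping BP_Tank, hiding the character and teleporting it to the world origin.
; Keys 1 and 2 cycle four isometric camera presets, setting a yaw offset that only sideways movement applies; forward uses plain control yaw.
; Legacy axis events remain as empty stubs with disconnected logic.
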(event Input|EnhancedActionEvents|EnhancedInputActionIA_Jump
  (params (ActionValue :type Boolean) (ElapsedSeconds :type Float%20%28double-precision%29) (TriggeredSeconds :type Float%20%28double-precision%29) (InputAction :type Input%20Action%20Object%20Reference :default "/Game/Blueprints/Character/IA_Jump.IA_Jump"))
  ;[0.15 0.15 0.15 0.5] JUMP U5
  (:Triggered
    (Character|Jump))
  (:Completed
    (Character|StopJumping)))

(event Input|EnhancedActionEvents|EnhancedInputActionIA_Look
  (params (ActionValue :type Vector%202D%20Structure) (ElapsedSeconds :type Float%20%28double-precision%29) (TriggeredSeconds :type Float%20%28double-precision%29) (InputAction :type Input%20Action%20Object%20Reference :default "/Game/Blueprints/Character/IA_Look.IA_Look"))
  ;[0.15 0.15 0.15 0.5] CAMERA CONTROL U5
  (Pawn|Input|AddControllerYawInput (.x ActionValue))
  (Pawn|Input|AddControllerPitchInput (.y ActionValue)))

(event Input|EnhancedActionEvents|EnhancedInputActionIA_Move
  (params (ActionValue :type Vector%202D%20Structure) (ElapsedSeconds :type Float%20%28double-precision%29) (TriggeredSeconds :type Float%20%28double-precision%29) (InputAction :type Input%20Action%20Object%20Reference :default "/Game/Blueprints/Character/IA_Move.IA_Move"))
  (bind _returnvalue (Pawn|GetControlRotation :!class /Script/Engine.Pawn))
  ;[0.15 0.15 0.15 0.5] MOVEMENT INPUT U5
  (Pawn|Input|AddMovementInput (Math|Vector|GetRightVector (Math|Rotator|MakeRotator (.roll _returnvalue) 0.0 (+ (.yaw _returnvalue) (Variables|Default|GetCameraOffSet)))) (.x ActionValue) false)
  (Pawn|Input|AddMovementInput (Math|Vector|GetForwardVector (Math|Rotator|MakeRotator 0.0 0.0 (.yaw (Pawn|GetControlRotation :!class /Script/Engine.Pawn)))) (.y ActionValue) false))

(event Input|EnhancedActionEvents|EnhancedInputActionIA_Zoom
  (params (ActionValue :type Float%20%28double-precision%29) (ElapsedSeconds :type Float%20%28double-precision%29) (TriggeredSeconds :type Float%20%28double-precision%29) (InputAction :type Input%20Action%20Object%20Reference :default "/Game/Blueprints/Character/IA_Zoom.IA_Zoom"))
  (bind _springarm (Variables|Default|GetSpringArm))
  ;[0.15 0.1275 0 0.5] CAMARA ZOOM CLASE
  (Variables|/Script/Engine.SpringArmComponent|SetTargetArmLength _springarm (+ (* ActionValue (Variables|Default|GetzoomAmount)) (Variables|/Script/Engine.SpringArmComponent|GetTargetArmLength _springarm))))

(event Input|EnhancedActionEvents|EnhancedInputActionIA_Interact
  (params (ActionValue :type Boolean) (ElapsedSeconds :type Float%20%28double-precision%29) (TriggeredSeconds :type Float%20%28double-precision%29) (InputAction :type Input%20Action%20Object%20Reference :default "/Game/Blueprints/Character/IA_Interact.IA_Interact"))
  ;[0.15 0.15 0.15 0.5] ENTRA AL TANQUE
  (for _array_element (Collision|GetOverlappingActors "/Game/Blueprints/Vehicle/BP_Tank.BP_Tank_C" :!class /Script/Engine.Actor)
    (bind _asbp_tank (Utilities|Casting|CastToBP_Tank _array_element))
    (Rendering|SetActorHiddenInGame true)
    (Pawn|Possess (Game|GetPlayerController 0) _asbp_tank)
    (Transformation|SetActorLocation "0, 0, 0" false true)))

(event Input|EnhancedActionEvents|EnhancedInputActionIA_Run
  (params (ActionValue :type Float%20%28double-precision%29) (ElapsedSeconds :type Float%20%28double-precision%29) (TriggeredSeconds :type Float%20%28double-precision%29) (InputAction :type Input%20Action%20Object%20Reference :default "/Game/Blueprints/Character/IA_Run.IA_Run"))
  ;[0.15 0.1416 0 0.5] CAMERA SHAKE CLASE
  (:Triggered
    (Camera|PlayWorldCameraShake "/Game/Blueprints/BP_CameraShake.BP_CameraShake_C" (Transformation|GetActorLocation) 0.0 1e+04 0.0)
    ;[0.15 0.1374 0 0.5] RUN CLASE
    (Variables|/Script/Engine.CharacterMovementComponent|SetMaxWalkSpeed (Variables|Character|GetCharacterMovement) (Variables|Default|GetrunSpeed)))
  (:Completed
    (CameraShake|StopAllCameraShakes (Game|GetPlayerCameraManager 0) true)
    (Variables|/Script/Engine.CharacterMovementComponent|SetMaxWalkSpeed (Variables|Character|GetCharacterMovement) (Variables|Default|GetwalkSpeed))))

(event EventBeginPlay
  ;[0.15 0.15 0.15 0.5] CONTEXT MAPPING INSTANCE
  (bind _asplayer_controller (Utilities|Casting|CastToPlayerController (Pawn|GetController)))
  (Utilities|IsValid (PlayerController|LocalPlayerSubsystems|GetEnhancedInputLocalPlayerSubsystem _asplayer_controller)
    (:Is%20Valid
      (Input|AddMappingContext (PlayerController|LocalPlayerSubsystems|GetEnhancedInputLocalPlayerSubsystem _asplayer_controller) "/Game/Blueprints/IMC_MyGame.IMC_MyGame" 0 "(bIgnoreAllPressedKeysUntilRelease=True,bForceImmediately=False,bNotifyUserSettings=False)"))))

(event Input|AxisEvents|InputAxisForwardAxis
  (params (AxisValue :type Float%20%28single-precision%29))
  ;[0.15 0.001563 0.001563 0.5] MOVIMIENTO CLASE U4
)

(event Input|AxisEvents|InputAxisHorizontalAxis
  (params (AxisValue :type Float%20%28single-precision%29))
  ;[0.15 0.001563 0.001563 0.5] MOVIMIENTO CLASE U4
)

(event Input|AxisEvents|InputAxisTurn
  (params (AxisValue :type Float%20%28single-precision%29))
  ;[0.15 0 0 0.5] CAMARA CLASE U4
)

(event Input|AxisEvents|InputAxisLookUp
  (params (AxisValue :type Float%20%28single-precision%29))
  ;[0.15 0 0 0.5] CAMARA CLASE U4
)

(event Input|KeyboardEvents|1
  (params (Key :type Key%20Structure :default "None"))
  ;[0.15 0.15 0.15 0.5] Vista_Isometrica
  (:Released
    (if (== (Variables|Default|GetCameraPosition) 0)
      (Variables|Default|SetCameraPosition 3)
      (else
        (Math|Integer|DecrementInt (Variables|Default|GetCameraPosition)
          (:%20%20
            _))))
    (switch int (Variables|Default|GetCameraPosition)
      (:0
        (Variables|/Script/Engine.SpringArmComponent|SetTargetOffset (Variables|Default|GetSpringArm) "0.000000,400.000000,300.000000")
        (Transformation|SetRelativeRotation (Variables|Default|GetCamera) "-30.000000,-45.000000,0.000000" false false)
        (Variables|Default|SetCameraOffSet -45.0))
      (:1
        (Variables|/Script/Engine.SpringArmComponent|SetTargetOffset (Variables|Default|GetSpringArm) "800.000000,400.000000,300.000000")
        (Transformation|SetRelativeRotation (Variables|Default|GetCamera) "-30.000000,-135.000000,0.000000" false false)
        (Variables|Default|SetCameraOffSet -135.0))
      (:2
        (Variables|/Script/Engine.SpringArmComponent|SetTargetOffset (Variables|Default|GetSpringArm) "800.000000,-400.000000,300.000000")
        (Transformation|SetRelativeRotation (Variables|Default|GetCamera) "-30.000000,135.000000,0.000000" false false)
        (Variables|Default|SetCameraOffSet 135.0))
      (:3
        (Variables|/Script/Engine.SpringArmComponent|SetTargetOffset (Variables|Default|GetSpringArm) "0.000000,-400.000000,300.000000")
        (Transformation|SetRelativeRotation (Variables|Default|GetCamera) "-30.000000,45.000000,0.000000" false false)
        (Variables|Default|SetCameraOffSet 45.0)))))

(event Input|KeyboardEvents|2
  (params (Key :type Key%20Structure :default "None"))
  ;[0.15 0.15 0.15 0.5] Vista_Isometrica
  (:Released
    (if (== (Variables|Default|GetCameraPosition) 3)
      (Variables|Default|SetCameraPosition 0)
      (else
        (Math|Integer|IncrementInt (Variables|Default|GetCameraPosition)
          (:%20%20
            _))))
    (switch int (Variables|Default|GetCameraPosition)
      (:0
        (Variables|/Script/Engine.SpringArmComponent|SetTargetOffset (Variables|Default|GetSpringArm) "0.000000,400.000000,300.000000")
        (Transformation|SetRelativeRotation (Variables|Default|GetCamera) "-30.000000,-45.000000,0.000000" false false)
        (Variables|Default|SetCameraOffSet -45.0))
      (:1
        (Variables|/Script/Engine.SpringArmComponent|SetTargetOffset (Variables|Default|GetSpringArm) "800.000000,400.000000,300.000000")
        (Transformation|SetRelativeRotation (Variables|Default|GetCamera) "-30.000000,-135.000000,0.000000" false false)
        (Variables|Default|SetCameraOffSet -135.0))
      (:2
        (Variables|/Script/Engine.SpringArmComponent|SetTargetOffset (Variables|Default|GetSpringArm) "800.000000,-400.000000,300.000000")
        (Transformation|SetRelativeRotation (Variables|Default|GetCamera) "-30.000000,135.000000,0.000000" false false)
        (Variables|Default|SetCameraOffSet 135.0))
      (:3
        (Variables|/Script/Engine.SpringArmComponent|SetTargetOffset (Variables|Default|GetSpringArm) "0.000000,-400.000000,300.000000")
        (Transformation|SetRelativeRotation (Variables|Default|GetCamera) "-30.000000,45.000000,0.000000" false false)
        (Variables|Default|SetCameraOffSet 45.0)))))

(fn ConstructionScript)